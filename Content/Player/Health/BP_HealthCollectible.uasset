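; BP_HealthCollectible is a health pickup that appears as a randomly chosen food item.
; On BeginPlay it rolls a random index to set HealthMesh to an apple, watermelon or muffin, each paired with its own Heal amount.
; HealPlayerAmount returns that Heal value; the file itself contains no overlap or pickup logic.
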(event EventBeginPlay
  (bind _output_get (Variables|Default|SetNewVar (Math|Random|RandomIntegerinRange 0 2)))
  (if (== _output_get 0)
    (Components|StaticMesh|SetStaticMesh (Variables|Default|GetHealth%20Mesh) "/Game/Food_Pack_01/Meshes/Food_Fruit_Apple_01.Food_Fruit_Apple_01")
    (Variables|Default|SetHeal 1e+01)
    (elif (== _output_get 1)
      (Components|StaticMesh|SetStaticMesh (Variables|Default|GetHealth%20Mesh) "/Game/Food_Pack_01/Meshes/Food_Fruit_Watermelon_01.Food_Fruit_Watermelon_01")
      (Variables|Default|SetHeal 15.0)
      (else
        (Components|StaticMesh|SetStaticMesh (Variables|Default|GetHealth%20Mesh) "/Game/Food_Pack_01/Meshes/Food_Bread_Muffin_01.Food_Bread_Muffin_01")
        (Variables|Default|SetHeal 5.0)))))

(event EventDestroyed)

(fn ConstructionScript)

(fn HealPlayerAmount
  (return (Variables|Default|GetHeal)))